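; View delegate that animates match-3 explosion elements on spawn, drop, swap and match.
; Each event casts the accessor, queries it for locations and state, runs move/scale actions on the view's M3ViewActionsComponent, and reports completion through callback actions.
; Invalid swaps move back.
; Explosion matches chain two move-and-scale iterations, restore and reset, then join the normal match path, which pops and shrinks the view when matching is possible.
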(event Custom|OnDropEnded
  (Class|M3ElementViewAccessor|OnDropEnded (Variables|Default|GetAccessor)))

(event EventOnDrop
  (params (Accessor :type M3%20Element%20View%20Accessor%20Object%20Reference))
  (bind _duration (Variables|Default|GetDuration))
  (bind _asm3element_explosion_view_accessor_bp (Utilities|Casting|CastToM3ElementExplosionViewAccessor_BP Accessor))
  (bind _output_get (Variables|Default|SetAccessor _asm3element_explosion_view_accessor_bp))
  (bind _returnvalue (Class|M3ElementViewAccessor|GetCurrentLocation _output_get))
  (bind _returnvalue_2 (Class|M3ViewActionsComponent|MovetoAction (Actor|GetComponentbyClass (Variables|/Script/M3.M3ElementViewAccessor|GetView _output_get) "/Script/M3.M3ViewActionsComponent") _duration _returnvalue))
  (Class|M3ViewActionsComponent|RunAction (Actor|GetComponentbyClass (Variables|/Script/M3.M3ElementViewAccessor|GetView _output_get) "/Script/M3.M3ViewActionsComponent") _returnvalue_2)
  (bind _returnvalue_3 (Class|M3ViewActionsComponent|CallbackAction (Actor|GetComponentbyClass (Variables|/Script/M3.M3ElementViewAccessor|GetView _output_get) "/Script/M3.M3ViewActionsComponent") _duration (delegate Custom|OnDropEnded)))
  (Class|M3ViewActionsComponent|RunAction (Actor|GetComponentbyClass (Variables|/Script/M3.M3ElementViewAccessor|GetView _output_get) "/Script/M3.M3ViewActionsComponent") _returnvalue_3))

(event Custom|OnValidSwapEnd
  (bind _duration (Variables|Default|GetDuration))
  (bind _accessor (Variables|Default|GetAccessor))
  (bind _view (Variables|/Script/M3.M3ElementViewAccessor|GetView _accessor))
  (bind _returnvalue (Actor|GetComponentbyClass _view "/Script/M3.M3ViewActionsComponent"))
  (if (Variables|/Script/M3.M3ElementViewAccessor|GetIsPosibleToSwap _accessor)
    (Class|M3ElementViewAccessor|OnSwapEnded (Variables|Default|GetAccessor))
    (else
      (bind _returnvalue_2 (Class|M3ElementViewAccessor|GetCurrentLocation _accessor))
      (bind _returnvalue_3 (Class|M3ViewActionsComponent|MovetoAction _returnvalue _duration _returnvalue_2))
      (Class|M3ViewActionsComponent|RunAction _returnvalue _returnvalue_3)
      (bind _returnvalue_4 (Class|M3ViewActionsComponent|CallbackAction _returnvalue _duration (delegate Custom|OnInvalidSwapEnded)))
      (Class|M3ViewActionsComponent|RunAction _returnvalue _returnvalue_4))))

(event Custom|OnInvalidSwapEnded
  (Class|M3ElementViewAccessor|OnSwapEnded (Variables|Default|GetAccessor)))

(event EventOnSwap
  (params (Accessor :type M3%20Element%20View%20Accessor%20Object%20Reference))
  (bind _duration (Variables|Default|GetDuration))
  (bind _asm3element_explosion_view_accessor_bp (Utilities|Casting|CastToM3ElementExplosionViewAccessor_BP Accessor))
  (bind _output_get (Variables|Default|SetAccessor _asm3element_explosion_view_accessor_bp))
  (bind _returnvalue (Class|M3ElementViewAccessor|GetOppositeLocation _output_get))
  (bind _returnvalue_2 (Class|M3ViewActionsComponent|MovetoAction (Actor|GetComponentbyClass (Variables|/Script/M3.M3ElementViewAccessor|GetView _output_get) "/Script/M3.M3ViewActionsComponent") _duration _returnvalue))
  (Class|M3ViewActionsComponent|RunAction (Actor|GetComponentbyClass (Variables|/Script/M3.M3ElementViewAccessor|GetView _output_get) "/Script/M3.M3ViewActionsComponent") _returnvalue_2)
  (bind _returnvalue_3 (Class|M3ViewActionsComponent|CallbackAction (Actor|GetComponentbyClass (Variables|/Script/M3.M3ElementViewAccessor|GetView _output_get) "/Script/M3.M3ViewActionsComponent") _duration (delegate Custom|OnValidSwapEnd)))
  (Class|M3ViewActionsComponent|RunAction (Actor|GetComponentbyClass (Variables|/Script/M3.M3ElementViewAccessor|GetView _output_get) "/Script/M3.M3ViewActionsComponent") _returnvalue_3))

(event Custom|OnExplosionIteration1Ended
  (bind _duration (Variables|Default|GetDuration))
  (bind _returnvalue (Class|M3ElementExplosionViewAccessor|GetExplosionIteration2Location (Variables|Default|GetAccessor)))
  (bind _returnvalue_2 (Class|M3ViewActionsComponent|MovetoAction (Actor|GetComponentbyClass (Variables|/Script/M3.M3ElementViewAccessor|GetView (stale EventOnMatch _output_get)) "/Script/M3.M3ViewActionsComponent") _duration _returnvalue))
  (Class|M3ViewActionsComponent|RunAction (Actor|GetComponentbyClass (Variables|/Script/M3.M3ElementViewAccessor|GetView (stale EventOnMatch _output_get)) "/Script/M3.M3ViewActionsComponent") _returnvalue_2)
  (bind _returnvalue_3 (Class|M3ViewActionsComponent|ScaletoAction (Actor|GetComponentbyClass (Variables|/Script/M3.M3ElementViewAccessor|GetView (stale EventOnMatch _output_get)) "/Script/M3.M3ViewActionsComponent") _duration (Math|Vector|MakeVector 1.33 1.33 1.33)))
  (Class|M3ViewActionsComponent|RunAction (Actor|GetComponentbyClass (Variables|/Script/M3.M3ElementViewAccessor|GetView (stale EventOnMatch _output_get)) "/Script/M3.M3ViewActionsComponent") _returnvalue_3)
  (bind _returnvalue_4 (Class|M3ViewActionsComponent|CallbackAction (Actor|GetComponentbyClass (Variables|/Script/M3.M3ElementViewAccessor|GetView (stale EventOnMatch _output_get)) "/Script/M3.M3ViewActionsComponent") _duration (delegate Custom|OnExplosionIteration2Ended)))
  (Class|M3ViewActionsComponent|RunAction (Actor|GetComponentbyClass (Variables|/Script/M3.M3ElementViewAccessor|GetView (stale EventOnMatch _output_get)) "/Script/M3.M3ViewActionsComponent") _returnvalue_4))

(event Custom|OnMatchEnded
  (Class|M3ElementViewAccessor|OnMatchEnded (Variables|Default|GetAccessor)))

(event Custom|OnExplosionIteration2Ended
  (bind _duration (Variables|Default|GetDuration))
  (bind _accessor (Variables|Default|GetAccessor))
  (bind _returnvalue (Class|M3ElementViewAccessor|GetCurrentLocation _accessor))
  (bind _returnvalue_2 (Class|M3ViewActionsComponent|MovetoAction (Actor|GetComponentbyClass (Variables|/Script/M3.M3ElementViewAccessor|GetView (stale EventOnMatch _output_get)) "/Script/M3.M3ViewActionsComponent") _duration _returnvalue))
  (Class|M3ViewActionsComponent|RunAction (Actor|GetComponentbyClass (Variables|/Script/M3.M3ElementViewAccessor|GetView (stale EventOnMatch _output_get)) "/Script/M3.M3ViewActionsComponent") _returnvalue_2)
  (bind _returnvalue_3 (Class|M3ViewActionsComponent|ScaletoAction (Actor|GetComponentbyClass (Variables|/Script/M3.M3ElementViewAccessor|GetView (stale EventOnMatch _output_get)) "/Script/M3.M3ViewActionsComponent") _duration (Math|Vector|MakeVector 1.0 1.0 1.0)))
  (Class|M3ViewActionsComponent|RunAction (Actor|GetComponentbyClass (Variables|/Script/M3.M3ElementViewAccessor|GetView (stale EventOnMatch _output_get)) "/Script/M3.M3ViewActionsComponent") _returnvalue_3)
  (Class|M3ElementExplosionViewAccessor|Reset _accessor)
  (if (Variables|/Script/M3.M3ElementViewAccessor|GetIsPosibleToMatch (stale EventOnMatch _output_get))
    (bind _returnvalue_4 (Class|M3ViewActionsComponent|ScaletoAction (Actor|GetComponentbyClass (Variables|/Script/M3.M3ElementViewAccessor|GetView (stale EventOnMatch _output_get)) "/Script/M3.M3ViewActionsComponent") _duration (Math|Vector|MakeVector 1.25 1.25 1.25)))
    (Class|M3ViewActionsComponent|RunAction (Actor|GetComponentbyClass (Variables|/Script/M3.M3ElementViewAccessor|GetView (stale EventOnMatch _output_get)) "/Script/M3.M3ViewActionsComponent") _returnvalue_4)
    (bind _returnvalue_5 (Class|M3ViewActionsComponent|ScaletoAction (Actor|GetComponentbyClass (Variables|/Script/M3.M3ElementViewAccessor|GetView (stale EventOnMatch _output_get)) "/Script/M3.M3ViewActionsComponent") _duration (Math|Vector|MakeVector 0.1 0.1 0.1)))
    (Class|M3ViewActionsComponent|RunAction (Actor|GetComponentbyClass (Variables|/Script/M3.M3ElementViewAccessor|GetView (stale EventOnMatch _output_get)) "/Script/M3.M3ViewActionsComponent") _returnvalue_5))
  (bind _returnvalue_6 (Class|M3ViewActionsComponent|CallbackAction (Actor|GetComponentbyClass (Variables|/Script/M3.M3ElementViewAccessor|GetView (stale EventOnMatch _output_get)) "/Script/M3.M3ViewActionsComponent") _duration (delegate Custom|OnMatchEnded)))
  (Class|M3ViewActionsComponent|RunAction (Actor|GetComponentbyClass (Variables|/Script/M3.M3ElementViewAccessor|GetView (stale EventOnMatch _output_get)) "/Script/M3.M3ViewActionsComponent") _returnvalue_6))

(event EventOnMatch
  (params (Accessor :type M3%20Element%20View%20Accessor%20Object%20Reference))
  (bind _duration (Variables|Default|GetDuration))
  (bind _asm3element_explosion_view_accessor_bp (Utilities|Casting|CastToM3ElementExplosionViewAccessor_BP Accessor))
  (bind _output_get (Variables|Default|SetAccessor _asm3element_explosion_view_accessor_bp))
  (if (Variables|/Script/M3Game.M3ElementExplosionViewAccessor|GetIsExplosion _output_get)
    (bind _returnvalue (Class|M3ElementExplosionViewAccessor|GetExplosionIteration1Location (Variables|Default|GetAccessor)))
    (bind _returnvalue_2 (Class|M3ViewActionsComponent|MovetoAction (Actor|GetComponentbyClass (Variables|/Script/M3.M3ElementViewAccessor|GetView _output_get) "/Script/M3.M3ViewActionsComponent") _duration _returnvalue))
    (Class|M3ViewActionsComponent|RunAction (Actor|GetComponentbyClass (Variables|/Script/M3.M3ElementViewAccessor|GetView _output_get) "/Script/M3.M3ViewActionsComponent") _returnvalue_2)
    (bind _returnvalue_3 (Class|M3ViewActionsComponent|ScaletoAction (Actor|GetComponentbyClass (Variables|/Script/M3.M3ElementViewAccessor|GetView _output_get) "/Script/M3.M3ViewActionsComponent") _duration (Math|Vector|MakeVector 0.33 0.33 0.33)))
    (Class|M3ViewActionsComponent|RunAction (Actor|GetComponentbyClass (Variables|/Script/M3.M3ElementViewAccessor|GetView _output_get) "/Script/M3.M3ViewActionsComponent") _returnvalue_3)
    (bind _returnvalue_4 (Class|M3ViewActionsComponent|CallbackAction (Actor|GetComponentbyClass (Variables|/Script/M3.M3ElementViewAccessor|GetView _output_get) "/Script/M3.M3ViewActionsComponent") _duration (delegate Custom|OnExplosionIteration1Ended)))
    (Class|M3ViewActionsComponent|RunAction (Actor|GetComponentbyClass (Variables|/Script/M3.M3ElementViewAccessor|GetView _output_get) "/Script/M3.M3ViewActionsComponent") _returnvalue_4)
    (else
      (if (Variables|/Script/M3.M3ElementViewAccessor|GetIsPosibleToMatch _output_get)
        (bind _returnvalue_5 (Class|M3ViewActionsComponent|ScaletoAction (Actor|GetComponentbyClass (Variables|/Script/M3.M3ElementViewAccessor|GetView _output_get) "/Script/M3.M3ViewActionsComponent") _duration (Math|Vector|MakeVector 1.25 1.25 1.25)))
        (Class|M3ViewActionsComponent|RunAction (Actor|GetComponentbyClass (Variables|/Script/M3.M3ElementViewAccessor|GetView _output_get) "/Script/M3.M3ViewActionsComponent") _returnvalue_5)
        (bind _returnvalue_6 (Class|M3ViewActionsComponent|ScaletoAction (Actor|GetComponentbyClass (Variables|/Script/M3.M3ElementViewAccessor|GetView _output_get) "/Script/M3.M3ViewActionsComponent") _duration (Math|Vector|MakeVector 0.1 0.1 0.1)))
        (Class|M3ViewActionsComponent|RunAction (Actor|GetComponentbyClass (Variables|/Script/M3.M3ElementViewAccessor|GetView _output_get) "/Script/M3.M3ViewActionsComponent") _returnvalue_6))
      (bind _returnvalue_7 (Class|M3ViewActionsComponent|CallbackAction (Actor|GetComponentbyClass (Variables|/Script/M3.M3ElementViewAccessor|GetView _output_get) "/Script/M3.M3ViewActionsComponent") _duration (delegate Custom|OnMatchEnded)))
      (Class|M3ViewActionsComponent|RunAction (Actor|GetComponentbyClass (Variables|/Script/M3.M3ElementViewAccessor|GetView _output_get) "/Script/M3.M3ViewActionsComponent") _returnvalue_7))))

(event Custom|OnSpawnEnded
  (Class|M3ElementViewAccessor|OnSpawnEnded (Variables|Default|GetAccessor)))

(event EventOnSpawn
  (params (Accessor :type M3%20Element%20View%20Accessor%20Object%20Reference))
  (bind _duration (Variables|Default|GetDuration))
  (bind _asm3element_explosion_view_accessor_bp (Utilities|Casting|CastToM3ElementExplosionViewAccessor_BP Accessor))
  (bind _output_get (Variables|Default|SetAccessor _asm3element_explosion_view_accessor_bp))
  (bind _returnvalue (Class|M3ElementViewAccessor|GetCurrentLocation _output_get))
  (Transformation|SetActorLocation (Variables|/Script/M3.M3ElementViewAccessor|GetView _output_get) _returnvalue false false)
  (Transformation|SetActorScale3D (Variables|/Script/M3.M3ElementViewAccessor|GetView _output_get) "0, 0, 0")
  (bind _returnvalue_2 (Class|M3ViewActionsComponent|ScaletoAction (Actor|GetComponentbyClass (Variables|/Script/M3.M3ElementViewAccessor|GetView _output_get) "/Script/M3.M3ViewActionsComponent") _duration (Math|Vector|MakeVector 1.0 1.0 1.0)))
  (Class|M3ViewActionsComponent|RunAction (Actor|GetComponentbyClass (Variables|/Script/M3.M3ElementViewAccessor|GetView _output_get) "/Script/M3.M3ViewActionsComponent") _returnvalue_2)
  (bind _returnvalue_3 (Class|M3ViewActionsComponent|CallbackAction (Actor|GetComponentbyClass (Variables|/Script/M3.M3ElementViewAccessor|GetView _output_get) "/Script/M3.M3ViewActionsComponent") _duration (delegate Custom|OnSpawnEnded)))
  (Class|M3ViewActionsComponent|RunAction (Actor|GetComponentbyClass (Variables|/Script/M3.M3ElementViewAccessor|GetView _output_get) "/Script/M3.M3ViewActionsComponent") _returnvalue_3))