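; Match-3 HUD that creates the M3Menu widget on BeginPlay, adds it to the viewport and turns on the FPS stat display.
; Change events for goals, duration and score write formatted text into the widget's labels.
; Up to three color-collection goals map by index to their labels, and duration reads as turns or time depending on the mode.
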(event `self.OnGoalChanged`
  (params (Id :type "EM3GoalId Enum" :default "UNKNOWN") (Index :type Integer) (CurrentQuantity :type Integer) (MaxQuantity :type Integer))
  (bind _m3menu (`self.M3Menu`))
  (bind _result (`|FormatText` "Collect {0} elements: {1}/{2}" (`self.ElementColorText`) CurrentQuantity MaxQuantity))
  (bind _label_goala (`/Game/M3Menu_BP.Label_GoalA` _m3menu))
  (bind _label_goalb (`/Game/M3Menu_BP.Label_GoalB` _m3menu))
  (bind _label_goalc (`/Game/M3Menu_BP.Label_GoalC` _m3menu))
  (`/Engine/EditorBlueprintResources/StandardMacros.IsValid` (`self.M3Menu`)
    (:`Is Valid`
      (if (< Index 3)
        (switch `EM3GoalId` Id
          (:`COLLECT_RED_ELEMENTS`
            (set `self.ElementColorText` "Red"))
          (:`COLLECT_GREEN_ELEMENTS`
            (set `self.ElementColorText` "Green"))
          (:`COLLECT_BLUE_ELEMENTS`
            (set `self.ElementColorText` "Blue"))
          (:`COLLECT_YELLOW_ELEMENTS`
            (set `self.ElementColorText` "Yellow"))
          (:`COLLECT_ORANGE_ELEMENTS`
            (set `self.ElementColorText` "Orange"))
          (:`COLLECT_PURPLE_ELEMENTS`
            (set `self.ElementColorText` "Purple")))
        (switch `int` Index
          (:`0`
            (`/Engine/EditorBlueprintResources/StandardMacros.IsValid` _label_goala
              (:`Is Valid`
                (`TextBlock.SetText` _label_goala _result))))
          (:`1`
            (`/Engine/EditorBlueprintResources/StandardMacros.IsValid` _label_goalb
              (:`Is Valid`
                (`TextBlock.SetText` _label_goalb _result))))
          (:`2`
            (`/Engine/EditorBlueprintResources/StandardMacros.IsValid` _label_goalc
              (:`Is Valid`
                (`TextBlock.SetText` _label_goalc _result)))))))))

(event `self.OnDurationChanged`
  (params (CurrentDuration :type Integer) (MaxDuration :type Integer) (IsTurnBased :type Boolean))
  (bind _m3menu (`self.M3Menu`))
  (bind _label_duration (`/Game/M3Menu_BP.Label_Duration` _m3menu))
  (`/Engine/EditorBlueprintResources/StandardMacros.IsValid` _m3menu
    (:`Is Valid`
      (if IsTurnBased
        (`TextBlock.SetText` _label_duration (`|FormatText` "Turns: {0}/{1}" CurrentDuration MaxDuration))
        (else
          (`TextBlock.SetText` _label_duration (`|FormatText` "Time: {0}/{1}" CurrentDuration MaxDuration)))))))

(event `self.OnScoresChanged`
  (params (CurrentScores :type Integer) (Star1Scores :type Integer) (Star2Scores :type Integer) (Star3Scores :type Integer))
  (bind _m3menu (`self.M3Menu`))
  (`/Engine/EditorBlueprintResources/StandardMacros.IsValid` _m3menu
    (:`Is Valid`
      (`TextBlock.SetText` (`/Game/M3Menu_BP.Label_Scores` _m3menu) (`|FormatText` "Scores: {0}" CurrentScores)))))

(event `self.ReceiveBeginPlay`
  (bind _returnvalue (`|CreateWidget` "/Game/M3Menu_BP.M3Menu_BP_C"))
  (`UserWidget.AddToViewport` _returnvalue 0)
  (set `self.M3Menu` _returnvalue)
  (`KismetSystemLibrary.ExecuteConsoleCommand` "stat FPS"))

(fn `UserConstructionScript`)