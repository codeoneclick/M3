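; View delegate that animates match-3 board elements for drop, swap, match and spawn events.
; Each event queues move or scale actions on the view's M3ViewActionsComponent, then a callback action reporting completion to the Accessor.
; Targets derive from row, column and element size relative to the parent actor.
; Invalid swaps move back before reporting, and spawn completion calls OnSwapEnded rather than a spawn-specific callback.
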(fn `GetCurrentLocation`
  (returns (Location :type "Vector Structure"))
  (bind _accessor (`self.Accessor`))
  (bind (_x _y) (`KismetMathLibrary.BreakVector2D` (`M3ElementViewAccessor.ElementSize` _accessor)))
  (return (`KismetMathLibrary.MakeVector` (+ (.x (`Actor.K2_GetActorLocation` (`Actor.GetAttachParentActor` (`M3ElementViewAccessor.View` _accessor)))) (`KismetMathLibrary.Conv_IntToDouble` (* (`M3ElementViewAccessor.CurrentRow` _accessor) (`KismetMathLibrary.FTrunc` _y)))) (+ (.y (`Actor.K2_GetActorLocation` (`Actor.GetAttachParentActor` (`M3ElementViewAccessor.View` _accessor)))) (`KismetMathLibrary.Conv_IntToDouble` (* (`M3ElementViewAccessor.CurrentCol` _accessor) (`KismetMathLibrary.FTrunc` _x)))))))

(fn `GetOpossiteLocation`
  (returns (Location :type "Vector Structure"))
  (bind _accessor (`self.Accessor`))
  (bind (_x _y) (`KismetMathLibrary.BreakVector2D` (`M3ElementViewAccessor.ElementSize` _accessor)))
  (return (`KismetMathLibrary.MakeVector` (+ (.x (`Actor.K2_GetActorLocation` (`Actor.GetAttachParentActor` (`M3ElementViewAccessor.View` _accessor)))) (`KismetMathLibrary.Conv_IntToDouble` (* (`M3ElementViewAccessor.OppositeRow` _accessor) (`KismetMathLibrary.FTrunc` _y)))) (+ (.y (`Actor.K2_GetActorLocation` (`Actor.GetAttachParentActor` (`M3ElementViewAccessor.View` _accessor)))) (`KismetMathLibrary.Conv_IntToDouble` (* (`M3ElementViewAccessor.OppositeCol` _accessor) (`KismetMathLibrary.FTrunc` _x)))))))